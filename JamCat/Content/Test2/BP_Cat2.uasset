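; Physics-driven cat that BP_Light2 steers, scoring as saved on touching BP_Earth2 or dead on touching BP_Enemy2.
; Each tick applies a distance-scaled force toward the light, reversed at close range and zeroed when a line trace hits BP_Enemy_Circle, plus screen-edge bounce impulses.
; Overlaps update BP_UI scores, trigger particles and destroy the cat, with a red camera flash on death.
; Lifespan timers close its eyes, then fade it out.
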(event OnComponentBeginOverlap(catgeo)
  (params (OverlappedComponent :type Primitive%20Component%20Object%20Reference) (OtherActor :type Actor%20Object%20Reference) (OtherComp :type Primitive%20Component%20Object%20Reference) (OtherBodyIndex :type Integer) (bFromSweep :type Boolean) (SweepResult :type Hit%20Result%20Structure%20%28by%20ref%29))
  (bind _returnvalue (Game|GetPlayerCameraManager 0))
  (bind _cat_art (Variables|Default|Getcat%20art))
  (bind _ui (Variables|Default|Getui))
  (bind _win_particle_scale (Variables|Default|Getwin%20particle%20scale))
  (bind _die_particle_scale (Variables|Default|Getdie%20particle%20scale))
  (bind _screen_red_flash_alpha (Variables|Default|Getscreen%20red%20flash%20alpha))
  (bind _struct_scores (Variables|/Game/Test2/BP_UI.BP_UI_C|Getstruct%20scores _ui))
  (bind (_savedcat _deadcat) (Utilities|Struct|BreakStruct_Scores _struct_scores))
  ;[1 1 1] death
  (Utilities|FlowControl|Sequence
    (:then_0
      (Utilities|Casting|CastToBP_Earth2 OtherActor)
      (if (not (Variables|Default|Getpending%20die))
        (Variables|Default|Setpending%20win true)
        ;;[1 1 1] score
        (bind _result (Math|Integer|IncrementInt _savedcat)
          (:%20%20
            (Default|ScorePulseDie _ui)
            (Utilities|Struct|SetmembersinStruct_Scores _struct_scores _result)
            (Utilities|FlowControl|DoOnce false
              (:Completed
                (Utilities|FlowControl|Sequence
                  (:then_1
                    (bind _1 (Timeline|Timeline_0 PlayFromStart)
                      (:Update
                        (Transformation|SetWorldScale3D _cat_art (* (Transformation|GetWorldScale _cat_art) _1)))
                      (:Finished
                        (Actor|DestroyActor))))
                  (:then_2
                    (Effects|SpawnEmitteratLocation "/Game/StarterContent/Particles/P_Sparks1.P_Sparks1" (Transformation|GetWorldLocation (Variables|Default|Getcat%20art)) "0, 0, 0" (Math|Vector|MakeVector _win_particle_scale _win_particle_scale _win_particle_scale))))))))))
    (:then_1
      (Utilities|Casting|CastToBP_Enemy2 OtherActor)
      (if (not (Variables|Default|Getpending%20win))
        (Variables|Default|Setpending%20die true)
        ;;[1 1 1] flash
        (CameraFades|StartCameraFade _returnvalue 0.0 _screen_red_flash_alpha 0.2 "(R=1.000000,G=0.000000,B=0.000000,A=1.000000)" false true)
        (CameraFades|StartCameraFade _returnvalue _screen_red_flash_alpha 0.0 0.2 "(R=1.000000,G=0.000000,B=0.000000,A=1.000000)" false true)
        (bind _result_2 (Math|Integer|IncrementInt _deadcat)
          (:%20%20
            (Default|ScorePulseWin _ui)
            (Utilities|Struct|SetmembersinStruct_Scores _struct_scores _result_2)
            (Utilities|FlowControl|DoOnce false
              (:Completed
                (Utilities|FlowControl|Sequence
                  (:then_1
                    (Effects|SpawnEmitteratLocation "/Game/StarterContent/Particles/P_Explosion1.P_Explosion1" (Transformation|GetWorldLocation (Variables|Default|Getcat%20art)) "0, 0, 0" (Math|Vector|MakeVector _die_particle_scale _die_particle_scale _die_particle_scale))
                    (Actor|DestroyActor)))))))))))

(event Custom|cat%20dying
  ;[1 1 1] dying
  (bind _1 (Timeline|Timeline_1 PlayFromStart)
    (:Update
      (Rendering|Material|SetScalarParameterValueonMaterials (Variables|Default|Getcat%20art) "Opacity Mask" _1))
    (:Finished
      (Actor|DestroyActor))))

(event Custom|cat%20fade%20in
  ;[1 1 1] fade in
  (bind _1 (Timeline|Timeline_2 PlayFromStart)
    (:Update
      (Rendering|Material|SetScalarParameterValueonMaterials (Variables|Default|Getcat%20art) "Opacity Mask" _1))))

(event Custom|cat%20close%20eyes
  ;[1 1 1] dying
  (Rendering|Material|SetScalarParameterValueonMaterials (Variables|Default|Getcat%20art) "frame" 1.0))

(event EventTick
  (params (DeltaSeconds :type Float%20%28single-precision%29))
  (bind _cat_geo (Variables|Default|Getcat%20geo))
  (bind _cat_geo_2 (Variables|Default|Getcat%20geo))
  (bind _light (Variables|Default|Getlight))
  (bind _cat_geo_3 (Variables|Default|Getcat%20geo))
  (bind _screen_edge_impulse (Variables|aboutscreenedges|Getscreen%20edge%20impulse))
  (bind _screen_half_x (Variables|aboutscreenedges|Getscreen%20half%20x))
  (bind _cat_geo_4 (Variables|Default|Getcat%20geo))
  (bind _returnvalue (Transformation|GetWorldLocation _cat_geo_2))
  (bind _returnvalue_2 (Transformation|GetWorldLocation _cat_geo))
  (bind _light_geo (Variables|/Game/Test2/BP_Light2.BP_Light2_C|Getlight%20geo _light))
  (bind _returnvalue_3 (Transformation|GetWorldLocation _light_geo))
  ;[1 1 1] time
  (Variables|Default|Setcur_time (+ DeltaSeconds (Variables|Default|Getcur_time)))
  (Utilities|FlowControl|Sequence
    (:then_0
      ;[1 1 1] cat light gravity vector
      (Variables|aboutforces|Setgravity%20vector (Math|Vector|Normalize (- _returnvalue_3 _returnvalue_2))))
    (:then_1
      ;[1 1 1] cat light distance
      (Variables|aboutforces|Setdistance (Math|Vector|Distance(Vector) _returnvalue_3 _returnvalue_2)))
    (:then_2
      ;[1 1 1] gravity
      (if (<= (Variables|aboutforces|Getdistance) 5e+02)
        (Physics|AddForce _cat_geo_4 (Math|Vector|NegateVector (* (* (Variables|aboutforces|Getgravity%20vector) (/ 1.0 (/ (Variables|aboutforces|Getdistance) 1e+04))) (Variables|aboutforces|Getgravity%20block%20factor))) "None" true)
        (else
          (Physics|AddForce _cat_geo_4 (* (* (Variables|aboutforces|Getgravity%20vector) (/ 1.0 (/ (Variables|aboutforces|Getdistance) 1e+04))) (Variables|aboutforces|Getgravity%20block%20factor)) "None" true))))
    (:then_3
      ;[1 1 1] screen edge bounce
      (if (>= (.y _returnvalue) _screen_half_x)
        (Physics|AddImpulse _cat_geo_3 (Math|Vector|MakeVector 0.0 (* _screen_edge_impulse -1.0) 0.0) "None" true)
        (elif (<= (.y _returnvalue) (* _screen_half_x -1.0))
          (Physics|AddImpulse _cat_geo_3 (Math|Vector|MakeVector 0.0 _screen_edge_impulse 0.0) "None" true))))
    (:then_4
      ;[1 1 1] show light gravity block
      (bind _outhit (Collision|LineTraceByChannel (Transformation|GetWorldLocation (Variables|Default|Getcat%20geo)) (Transformation|GetWorldLocation (Variables|/Game/Test2/BP_Light2.BP_Light2_C|Getlight%20geo (Variables|Default|Getlight))) "TraceTypeQuery1" false 0 "None"))
      (Utilities|Casting|CastToBP_Enemy_Circle (.HitActor (Collision|BreakHitResult _outhit))
        (:then
          (Variables|aboutforces|Setgravity%20block%20factor 0.0))
        (:CastFailed
          (Variables|aboutforces|Setgravity%20block%20factor (Variables|aboutforces|Getgravity%20scale%20amount)))))))

(event EventBeginPlay
  (bind _cat_lifespan (Variables|Default|Getcat%20lifespan))
  (Utilities|FlowControl|Sequence
    (:then_0
      (Variables|Default|Setpending%20win false)
      (Variables|Default|Setpending%20die false))
    (:then_1
      (bind _returnvalue (Actor|GetActorOfClass "/Game/Test2/BP_Light2.BP_Light2_C"))
      (Variables|Default|Setlight _returnvalue)
      (bind _returnvalue_2 (Actor|GetActorOfClass "/Game/Test2/BP_UI.BP_UI_C"))
      (Variables|Default|Setui _returnvalue_2)
      ;[1 1 1] dying
      (Utilities|Time|SetTimerbyEvent (delegate Custom|cat%20dying) _cat_lifespan)
      (Utilities|Time|SetTimerbyEvent (delegate Custom|cat%20close%20eyes) (- _cat_lifespan 5.0)))))

(fn ConstructionScript)