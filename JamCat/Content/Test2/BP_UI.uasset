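; BP_UI is an in-world score display actor that pulses one of two text render components on a die or win event.
; On BeginPlay it gives each text component its own dynamic material instance of the default opaque text material.
; The scorepulsedie and scorepulsewin events each restart a timeline that drives the "intensity" scalar on the first and second component's material, respectively.
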(event Custom|score%20pulse%20win
  (bind _1 (Timeline|Timeline_1 PlayFromStart)
    (:Update
      (Rendering|Material|SetScalarParameterValue (Variables|Default|Getdmi2) "intensity" _1 :!class /Script/Engine.MaterialInstanceDynamic))))

(event Custom|score%20pulse%20die
  (bind _1 (Timeline|Timeline_0 PlayFromStart)
    (:Update
      (Rendering|Material|SetScalarParameterValue (Variables|Default|Getdmi1) "intensity" _1 :!class /Script/Engine.MaterialInstanceDynamic))))

(event EventBeginPlay
  (bind _returnvalue (Rendering|Material|CreateDynamicMaterialInstance (Variables|Default|GetTextRender) 0 "/Game/DefaultTextMaterialOpaque_Inst.DefaultTextMaterialOpaque_Inst" "None" :!class /Script/Engine.PrimitiveComponent))
  (Variables|Default|Setdmi1 _returnvalue)
  (bind _returnvalue_2 (Rendering|Material|CreateDynamicMaterialInstance (Variables|Default|GetTextRender1) 0 "/Game/DefaultTextMaterialOpaque_Inst.DefaultTextMaterialOpaque_Inst" "None" :!class /Script/Engine.PrimitiveComponent))
  (Variables|Default|Setdmi2 _returnvalue_2))

(event Collision|EventActorBeginOverlap
  (params (OtherActor :type Actor%20Object%20Reference)))

(event EventTick
  (params (DeltaSeconds :type Float%20%28single-precision%29)))

(fn ConstructionScript)