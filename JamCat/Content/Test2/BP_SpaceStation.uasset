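; BP_SpaceStation is a space station actor that spins and periodically spits out BP_Cat2 actors.
; Tick accumulates scaled time into CurTime, which directly sets the station mesh's yaw.
; A modulo check on CurTime with a DoOnce spawns one cat per cycle, with random roll and a random-direction velocity impulse.
; Circular-movement and radial-impulse nodes are left unconnected.
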(event EventBeginPlay)

(event Collision|EventActorBeginOverlap
  (params (OtherActor :type Actor%20Object%20Reference)))

(event EventTick
  (params (DeltaSeconds :type Float%20%28single-precision%29))
  (bind _returnvalue (Transformation|GetActorTransform))
  (Utilities|FlowControl|Sequence
    (:then_0
      (bind _output_get (Variables|Default|Setcur_time (+ (* DeltaSeconds (Variables|Default|Getspd%20sacle)) (Variables|Default|Getcur_time))))
      (Utilities|FlowControl|Sequence
        (:then_0
          (Transformation|SetRelativeRotation (Variables|Default|Getspace_station) (Math|Rotator|MakeRotator 0.0 0.0 _output_get) false false))))
    (:then_1
      (if (>= (Math|Float|%(Float) (Variables|Default|Getcur_time) 2e+01) 1e+01)
        (Utilities|FlowControl|DoOnce false :!label _label
          (:Completed
            (bind _returnvalue_2 (Game|SpawnActorfromClass "/Game/Test2/BP_Cat2.BP_Cat2_C" (Math|Transform|MakeTransform (Math|Vector|MakeVector 0.0 (.y (.location _returnvalue)) (.z (.location _returnvalue))) (Math|Rotator|MakeRotator (Math|Random|RandomFloatinRange -2e+01 2e+01) 0.0 0.0) "1,1,1") "Undefined" 0 0))
            (Physics|AddImpulse (Variables|/Game/Test2/BP_Cat2.BP_Cat2_C|Getgeo _returnvalue_2) (* (Math|Random|RandomUnitVector) (Math|Random|RandomFloatinRange 5e+02 1e+03)) "None" true)))
        (else
          (goto _label Reset))))))

(fn ConstructionScript)