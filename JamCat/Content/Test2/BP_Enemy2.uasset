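; BP_Enemy2 is an enemy actor that circles on the Y-Z plane relative to BP_Earth2 and expires after a random lifetime.
; Construction picks a random mesh and rotation; BeginPlay randomizes speed, caches Earth's location and starts the death timer.
; Tick drives sine/cosine motion with SpawnZOffset as radius, offset in Z from the cached center.
; Death disables collision, fades Opacity Mask by timeline, then destroys the actor; several older movement and randomization chains are disconnected.
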(event Custom|die
  (Collision|SetCollisionEnabled (Variables|Default|GetStaticMesh) "NoCollision")
  (bind _1 (Timeline|Timeline_0 Play)
    (:Update
      (Rendering|Material|SetScalarParameterValueonMaterials (Variables|Default|Getmesh) "Opacity Mask" _1))
    (:Finished
      (Actor|DestroyActor))))

(event EventBeginPlay
  (bind _life_range (Variables|Default|Getlife%20range))
  (bind _spd_range (Variables|Default|Getspd%20range))
  (Utilities|FlowControl|Sequence
    (:then_0
      (Utilities|Time|SetTimerbyEvent (delegate Custom|die) (Math|Random|RandomFloatinRange (.x _life_range) (.y _life_range)) true))
    (:then_1
      (bind _returnvalue (Actor|GetActorOfClass "/Game/Test2/BP_Earth2.BP_Earth2_C"))
      (Variables|Default|Setearth%20center (Transformation|GetActorLocation _returnvalue)))
    (:then_2
      (Variables|Default|Setrandom%20spd (Math|Random|RandomFloatinRange (.x _spd_range) (.y _spd_range))))))

(event EventTick
  (params (DeltaSeconds :type Float%20%28single-precision%29))
  (bind _earth_center (Variables|Default|Getearth%20center))
  (bind _spawn_z_offset (Variables|Default|Getspawn%20z%20offset))
  (Utilities|FlowControl|Sequence
    (:then_0
      (Variables|Default|Setcur_time (+ (* DeltaSeconds (Variables|Default|Getrandom%20spd)) (Variables|Default|Getcur_time)))
      (Utilities|FlowControl|Sequence
        (:then_0
          (Transformation|SetActorLocation (Math|Vector|MakeVector (.x (Transformation|GetActorLocation)) (- (.y _earth_center) (* _spawn_z_offset (Math|Trig|Sin(Radians) (Variables|Default|Getcur_time)))) (+ (+ (- (.z _earth_center) (* _spawn_z_offset (Math|Trig|Cos(Radians) (Variables|Default|Getcur_time)))) _spawn_z_offset) (.z _earth_center))) false false))))))

(fn ConstructionScript
  (Transformation|SetRelativeRotation (Variables|Default|Getmesh) (Math|Random|RandomRotator false) false false)
  (Components|StaticMesh|SetStaticMesh (Variables|Default|Getmesh) (Utilities|Array|Get(acopy) (Variables|Default|Getmeshes) (Math|Random|RandomIntegerinRange 0 3))))