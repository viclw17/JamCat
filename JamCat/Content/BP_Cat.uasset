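; BP_Cat is a physics-driven cat that gets pulled toward the BP_Light in the level.
; Each Tick it applies a mass-independent force toward the light, inversely proportional to distance.
; A visibility trace to the light switches that pull off while a BP_Enemy_Circle blocks it.
; Overlapping an enemy circle fades the camera red until overlap ends; orbit movement, randomization and debug logic are left unconnected.
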(event OnComponentBeginOverlap(cat)
  (params (OverlappedComponent :type Primitive%20Component%20Object%20Reference) (OtherActor :type Actor%20Object%20Reference) (OtherComp :type Primitive%20Component%20Object%20Reference) (OtherBodyIndex :type Integer) (bFromSweep :type Boolean) (SweepResult :type Hit%20Result%20Structure%20%28by%20ref%29))
  (Utilities|Casting|CastToBP_Enemy_Circle OtherActor)
  (CameraFades|StartCameraFade (Game|GetPlayerCameraManager 0) 0.0 (Variables|Default|Getscreen%20red%20alpha) 0.5 "(R=1.000000,G=0.000000,B=0.000000,A=1.000000)" false true))

(event OnComponentHit(cat)
  (params (HitComponent :type Primitive%20Component%20Object%20Reference) (OtherActor :type Actor%20Object%20Reference) (OtherComp :type Primitive%20Component%20Object%20Reference) (NormalImpulse :type Vector :default "0, 0, 0") (Hit :type Hit%20Result%20Structure%20%28by%20ref%29)))

(event OnComponentEndOverlap(cat)
  (params (OverlappedComponent :type Primitive%20Component%20Object%20Reference) (OtherActor :type Actor%20Object%20Reference) (OtherComp :type Primitive%20Component%20Object%20Reference) (OtherBodyIndex :type Integer))
  (Utilities|Casting|CastToBP_Enemy_Circle OtherActor)
  (CameraFades|StartCameraFade (Game|GetPlayerCameraManager 0) (Variables|Default|Getscreen%20red%20alpha) 0.0 0.5 "(R=1.000000,G=0.000000,B=0.000000,A=1.000000)" false true))

(event EventTick
  (params (DeltaSeconds :type Float%20%28single-precision%29))
  (bind _cat (Variables|Default|Getcat))
  (bind _light (Variables|Default|Getlight))
  (bind _returnvalue (Transformation|GetWorldLocation _cat))
  (bind _sphere (Variables|/Game/BP_Light.BP_Light_C|GetSphere _light))
  (bind _returnvalue_2 (Transformation|GetWorldLocation _sphere))
  (Utilities|FlowControl|Sequence
    (:then_0
      (Variables|Default|Setcur_time (+ (* DeltaSeconds (Variables|Default|Getspd%20sacle%20random)) (Variables|Default|Getcur_time)))
      (Utilities|FlowControl|Sequence
        (:then_0)
        (:then_1
          (Variables|Default|Setgravity%20vector (Math|Vector|Normalize (- _returnvalue_2 _returnvalue))))
        (:then_2
          (Variables|Default|Setdistance (Math|Vector|Distance(Vector) _returnvalue_2 _returnvalue)))
        (:then_3
          (Physics|AddForce (Variables|Default|Getcat) (* (* (Variables|Default|Getgravity%20vector) (/ 1.0 (/ (Variables|Default|Getdistance) 1e+03))) (Variables|Default|Getforce%20scale)) "None" true))
        (:then_4
          (bind _outhit (Collision|LineTraceByChannel (Transformation|GetWorldLocation (Variables|Default|Getcat)) (Transformation|GetWorldLocation (Variables|/Game/BP_Light.BP_Light_C|GetSphere (Variables|Default|Getlight))) "TraceTypeQuery1" false 0 "ForOneFrame"))
          (Utilities|Casting|CastToBP_Enemy_Circle (.HitActor (Collision|BreakHitResult _outhit))
            (:then
              (Variables|Default|Setforce%20scale 0.0))
            (:CastFailed
              (Variables|Default|Setforce%20scale 2e+02))))))))

(event EventBeginPlay
  (bind _returnvalue (Actor|GetActorOfClass "/Game/BP_Light.BP_Light_C"))
  (Variables|Default|Setlight _returnvalue))

(fn ConstructionScript)