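; BP_Enemy_Circle is an enemy Blueprint whose static mesh moves in a circular path in the world YZ plane.
; Tick accumulates time and adds sine and cosine offsets scaled by R to the mesh's current location, so motion is cumulative and frame-rate dependent.
; The construction script multiplies the mesh's X and Z scale by one random factor for size variation, leaving Y unchanged.
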(event EventBeginPlay)

(event EventTick
  (params (DeltaSeconds :type Float%20%28single-precision%29))
  (bind _r (Variables|Default|Getr))
  (bind _staticmesh (Variables|Default|GetStaticMesh))
  (bind _returnvalue (Transformation|GetWorldLocation _staticmesh))
  (Variables|Default|Setcur_time (+ DeltaSeconds (Variables|Default|Getcur_time)))
  (Utilities|FlowControl|Sequence
    (:then_0
      (Transformation|SetWorldLocation _staticmesh (Math|Vector|MakeVector (.x _returnvalue) (+ (* _r (Math|Trig|Sin(Radians) (Variables|Default|Getcur_time))) (.y _returnvalue)) (+ (* _r (Math|Trig|Cos(Radians) (Variables|Default|Getcur_time))) (.z _returnvalue))) false false))))

(event Collision|EventActorBeginOverlap
  (params (OtherActor :type Actor%20Object%20Reference)))

(fn ConstructionScript
  (bind _staticmesh (Variables|Default|GetStaticMesh))
  (bind _returnvalue (Transformation|GetWorldScale _staticmesh))
  (Variables|Default|Setrandom (Math|Random|RandomFloatinRange 0.5 1.5))
  (Transformation|SetWorldScale3D _staticmesh (Math|Vector|MakeVector (* (.x _returnvalue) (Variables|Default|Getrandom)) (.y _returnvalue) (* (.z _returnvalue) (Variables|Default|Getrandom)))))